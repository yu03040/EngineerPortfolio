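; BP_FloorTile is a track segment for an endless runner that spawns with either one blocker or three coins, chosen randomly in its construction script.
; Blockers use one of three spawn points; coins land randomly inside the CoinArea box.
; When the runner overlaps EndTrigger, the game mode adds a tile and this one self-destructs after a delay.
; Side-wall hits kill the runner when the hit normal aligns with its forward vector.
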(event OnComponentBeginOverlap(EndTrigger)
  (params (OverlappedComponent :type Primitive%20Component%20Object%20Reference) (OtherActor :type Actor%20Object%20Reference) (OtherComp :type Primitive%20Component%20Object%20Reference) (OtherBodyIndex :type Integer) (bFromSweep :type Boolean) (SweepResult :type Hit%20Result%20Structure%20%28by%20ref%29))
  (Utilities|Casting|CastToBP_RunCharacter OtherActor) ; トリガーに来たのはランキャラクターか？
  (bind _asbp_run_game_mode (Utilities|Casting|CastToBP_RunGameMode (Game|GetGameMode)))
  (Default|AddFloorTile _asbp_run_game_mode)
  (Utilities|FlowControl|Delay 2.0)
  (Actor|DestroyActor) ; 増えていくから消す
)

(event OnComponentHit(SM_Crypt_Wall_Left_00)
  (params (HitComponent :type Primitive%20Component%20Object%20Reference) (OtherActor :type Actor%20Object%20Reference) (OtherComp :type Primitive%20Component%20Object%20Reference) (NormalImpulse :type Vector :default "0, 0, 0") (Hit :type Hit%20Result%20Structure%20%28by%20ref%29))
  (bind _asbp_run_character (Utilities|Casting|CastToBP_RunCharacter OtherActor))
  (if (Math|Float|NearlyEqual(Float) (Math|Vector|DotProduct (.normal Hit) (Math|Vector|GetForwardVector (Variables|/Script/Engine.Actor|GetRootComponent _asbp_run_character))) 1.0 0.01)
    (Default|Death _asbp_run_character)))

(event OnComponentHit(SM_Crypt_Wall_Right_00)
  (params (HitComponent :type Primitive%20Component%20Object%20Reference) (OtherActor :type Actor%20Object%20Reference) (OtherComp :type Primitive%20Component%20Object%20Reference) (NormalImpulse :type Vector :default "0, 0, 0") (Hit :type Hit%20Result%20Structure%20%28by%20ref%29))
  (bind _asbp_run_character (Utilities|Casting|CastToBP_RunCharacter OtherActor))
  (if (Math|Float|NearlyEqual(Float) (Math|Vector|DotProduct (.normal Hit) (Math|Vector|GetForwardVector (Variables|/Script/Engine.Actor|GetRootComponent _asbp_run_character))) 1.0 0.01)
    (Default|Death _asbp_run_character)))

(fn ConstructionScript
  (CallFunction|SetSpawnPoint)
  (switch int (Math|Random|RandomIntegerinRange 0 1)
    (:Default
      (CallFunction|SpawnBlocker :!label _label))
    (:0
      (goto _label))
    (:1
      (CallFunction|SpawnCoins))))

(fn GetAttachPoint
  (return (Transformation|GetWorldTransform (Variables|Default|GetAttachPoint))))

(fn SetSpawnPoint
  (Variables|Default|SetSpawnPoints (Utilities|Array|MakeArray (Transformation|GetRelativeTransform (Variables|Default|GetSpawnPointRight)) (Transformation|GetRelativeTransform (Variables|Default|GetSpawnPointLeft)) (Transformation|GetRelativeTransform (Variables|Default|GetSpawnPoint)))))

(fn SpawnBlocker
  (bind _spawnpoints (Variables|Default|GetSpawnPoints))
  (AddComponent|AddChildActorComponent false (Utilities|Array|Get(acopy) _spawnpoints (Math|Random|RandomIntegerinRange 0 (Utilities|Array|LastIndex _spawnpoints)))) ; 床と一緒に障害物を生成
)

(fn SpawnCoins
  (bind _coinarea (Variables|Default|GetCoinArea))
  (for _index (range 0 2) ; 3こ生成
    (AddComponent|AddChildActorComponent false (Math|Conversions|ToTransform(Vector) (Math|Random|RandomPointinBoundingBox (Variables|/Script/Engine.SceneComponent|GetRelativeLocation _coinarea) (Variables|/Script/Engine.BoxComponent|GetBoxExtent _coinarea)))) ; 床と一緒にコインを生成
  ))