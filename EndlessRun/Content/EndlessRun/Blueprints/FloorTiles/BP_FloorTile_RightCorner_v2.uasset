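; Right-corner floor tile for an endless runner, where the player character can turn.
; Hits on two wall meshes kill the character when the hit normal nearly matches its forward vector, so only head-on impacts count.
; Overlapping TurnZone sets CanTurn on the character.
; The construction script calls SpawnCoins, which adds three child actors at random points inside the CoinArea box.
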(event OnComponentHit(SM_Crypt_Wall_Left_00)
  (params (HitComponent :type Primitive%20Component%20Object%20Reference) (OtherActor :type Actor%20Object%20Reference) (OtherComp :type Primitive%20Component%20Object%20Reference) (NormalImpulse :type Vector :default "0, 0, 0") (Hit :type Hit%20Result%20Structure%20%28by%20ref%29))
  (bind _asbp_run_character_v_2 (Utilities|Casting|CastToBP_RunCharacter_v2 OtherActor))
  (if (Math|Float|NearlyEqual(Float) (Math|Vector|DotProduct (.Normal (Collision|BreakHitResult Hit)) (Math|Vector|GetForwardVector (Variables|/Script/Engine.Actor|GetRootComponent _asbp_run_character_v_2))) 1.0 0.01)
    (Default|Death _asbp_run_character_v_2)))

(event OnComponentHit(SM_Crypt_Wall_Floor_Trim_01)
  (params (HitComponent :type Primitive%20Component%20Object%20Reference) (OtherActor :type Actor%20Object%20Reference) (OtherComp :type Primitive%20Component%20Object%20Reference) (NormalImpulse :type Vector :default "0, 0, 0") (Hit :type Hit%20Result%20Structure%20%28by%20ref%29))
  (bind _asbp_run_character_v_2 (Utilities|Casting|CastToBP_RunCharacter_v2 OtherActor))
  (if (Math|Float|NearlyEqual(Float) (Math|Vector|DotProduct (.Normal (Collision|BreakHitResult Hit)) (Math|Vector|GetForwardVector (Variables|/Script/Engine.Actor|GetRootComponent _asbp_run_character_v_2))) 1.0 0.01)
    (Default|Death _asbp_run_character_v_2)))

(event OnComponentBeginOverlap(TurnZone)
  (params (OverlappedComponent :type Primitive%20Component%20Object%20Reference) (OtherActor :type Actor%20Object%20Reference) (OtherComp :type Primitive%20Component%20Object%20Reference) (OtherBodyIndex :type Integer) (bFromSweep :type Boolean) (SweepResult :type Hit%20Result%20Structure%20%28by%20ref%29))
  ;[0 0 0] 曲がれるようにCanTurnをセット
  (bind _asbp_run_character_v_2 (Utilities|Casting|CastToBP_RunCharacter_v2 OtherActor))
  (Variables|/Script/EndlessRun.RunCharacter|SetbCanTurn _asbp_run_character_v_2 true))

(event EventSpawnCoins
  (bind _coinarea (Variables|Default|GetCoinArea))
  (for _index (range 0 2)
    (AddComponent|AddChildActorComponent false (Math|Conversions|ToTransform(Vector) (Math|Random|RandomPointinBoundingBox (Variables|/Script/Engine.SceneComponent|GetRelativeLocation _coinarea) (Variables|/Script/Engine.BoxComponent|GetBoxExtent _coinarea))))))

(fn ConstructionScript
  (Class|FloorTileBase|SpawnCoins))