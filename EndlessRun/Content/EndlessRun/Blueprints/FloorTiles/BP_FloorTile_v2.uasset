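; BP_FloorTile_v2 is a floor tile for the endless runner that populates itself with a blocker and coins through child actor components.
; Construction calls SetSpawnPoint, whose body is not shown here.
; SpawnBlocker adds a child actor at a randomly picked SpawnPoints transform.
; SpawnCoins adds several child actors at random points inside the CoinArea box, using its relative location and extent.
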(event EventSpawnBlocker
  (bind _spawnpoints (Variables|Default|GetSpawnPoints))
  (AddComponent|AddChildActorComponent false (Utilities|Array|Get(acopy) _spawnpoints (Math|Random|RandomIntegerinRange 0 (Utilities|Array|LastIndex _spawnpoints)))))

(event EventSpawnCoins
  (bind _coinarea (Variables|Default|GetCoinArea))
  (for _index (range 0 2)
    (AddComponent|AddChildActorComponent false (Math|Conversions|ToTransform(Vector) (Math|Random|RandomPointinBoundingBox (Variables|/Script/Engine.SceneComponent|GetRelativeLocation _coinarea) (Variables|/Script/Engine.BoxComponent|GetBoxExtent _coinarea))))))

(fn ConstructionScript
  (Class|FloorTileBase|SetSpawnPoint))