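; Game mode for an endless runner that builds the track and tracks coins, distance and saved rankings.
; BeginPlay shows the score widget and pre-spawns random tiles, chaining each at the previous attach point and inserting a curve after a run of straights.
; Tick derives distance from scaled elapsed time and player forward vector, not actual displacement.
; ShowResult stops ticking and passes this run plus loaded SaveGame rankings to the result widget.
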(event Custom|ShowResult
  (Utilities|FlowControl|Sequence
    (:then_0
      (Variables|/Script/Engine.PlayerController|SetbShowMouseCursor (Game|GetPlayerController 0) true))
    (:then_1
      (Actor|Tick|SetActorTickEnabled false)
      (bind _return (CallFunction|LoadData))
      (bind _returnvalue (UserInterface|CreateWidget "/Game/EndlessRun/Blueprints/UMG/old/WBP_Result.WBP_Result_C" 0 (Utilities|Struct|MakeS_RankingData (Variables|Default|GetTotalCoins) (Variables|Default|GetSum%20Distance)) _return))
      (UserInterface|Viewport|AddtoViewport _returnvalue 0))))

(event EventBeginPlay
  (bind _returnvalue (UserInterface|CreateWidget "/Game/EndlessRun/Blueprints/UMG/old/WBP_RunScore.WBP_RunScore_C"))
  (UserInterface|Viewport|AddtoViewport _returnvalue 0)
  (for _index (range 0 10) ; 10回ループ
    (CallFunction|AddFloorTile)))

(event EventTick
  (params (DeltaSeconds :type Float%20%28single-precision%29))
  (CallFunction|RunDistance DeltaSeconds))

(fn ConstructionScript)

(fn AddFloorTile
  (if (> (Variables|Default|GetCurrentStraights) 7)
    (CallFunction|AddFloorTileCurve)
    (else
      (bind _returnvalue (Game|SpawnActorfromClass (Utilities|Array|Get(acopy) (Variables|Default|GetFloorTiles) (Math|Random|RandomIntegerinRange 0 (Utilities|Array|LastIndex (Variables|Default|GetFloorTiles)))) (Variables|Default|GetNextAttachPoint) "Undefined" "SelectDefaultAtRuntime" 0 0)) ; 床をランダムに生成
      (bind _asbp_floor_tile (Utilities|Casting|CastToBP_FloorTile _returnvalue)) ; フロアタイルだったら
      (bind _attachpoint (Default|GetAttachPoint _asbp_floor_tile)) ; Arrowをさがして
      (Variables|Default|SetNextAttachPoint _attachpoint) ; 更新しておく
      (Variables|Default|SetCurrentStraights (+ (Variables|Default|GetCurrentStraights) 1)))))

(fn AddFloorTileCurve
  (bind _floorcurves (Variables|Default|GetFloorCurves))
  (bind _returnvalue (Game|SpawnActorfromClass (Utilities|Array|Get(acopy) _floorcurves (Math|Random|RandomIntegerinRange 0 (Utilities|Array|LastIndex _floorcurves))) (Variables|Default|GetNextAttachPoint) "Undefined" "SelectDefaultAtRuntime" 0 0)) ; 床をランダムに生成
  (bind _asbp_floor_tile (Utilities|Casting|CastToBP_FloorTile _returnvalue)) ; フロアタイルだったら
  (bind _attachpoint (Default|GetAttachPoint _asbp_floor_tile)) ; Arrowをさがして
  (Variables|Default|SetNextAttachPoint _attachpoint) ; 更新しておく
  (Variables|Default|SetCurrentStraights 0) ; この関数が呼ばれたら0にしておく
)

(fn RunDistance
  (params (DeltaSeconds :type Float%20%28double-precision%29))
  ;[0 0 0] 1フレーム=(1/30)[s]だから(1/30)*30=1秒にして1秒ずつ足していく
  (Variables|Default|SetMoveSeconds (+ (* DeltaSeconds 3e+01) (Variables|Default|GetMoveSeconds)))
  (bind _asbp_run_character (Utilities|Casting|CastToBP_RunCharacter (Game|Player|GetPlayerPawn 0)))
  (Variables|Default|SetSum%20Distance (Math|Vector|VectorLengthXY (* (Variables|Default|GetMoveSeconds) (Transformation|GetActorForwardVector _asbp_run_character)))))

(fn AddCoin
  (Variables|Default|SetTotalCoins (+ (Variables|Default|GetTotalCoins) 1)))

(fn SaveData
  (params (NewRankingData :type Array%20of%20S%20Ranking%20Data%20Structures))
  (Variables|Default|SetNew%20Ranking%20Data NewRankingData)
  (bind _returnvalue (SaveGame|CreateSaveGameObject "/Game/EndlessRun/Blueprints/SaveGame/old/BP_SaveGame.BP_SaveGame_C"))
  (Variables|Default|SetSaveGameRef _returnvalue)
  (for _array_element (Variables|Default|GetNew%20Ranking%20Data)
    (Utilities|Array|Add (Variables|/Game/EndlessRun/Blueprints/SaveGame/old/BP_SaveGame.BP_SaveGame_C|GetRankingData (Variables|Default|GetSaveGameRef)) _array_element))
  (SaveGame|SaveGametoSlot (Variables|Default|GetSaveGameRef) (Variables|Default|GetSaveSlotName) (Variables|Default|GetSaveUserIndex)))

(fn LoadData
  (bind _returnvalue (SaveGame|LoadGamefromSlot (Variables|Default|GetSaveSlotName) (Variables|Default|GetSaveUserIndex)))
  (bind _asbp_save_game (Utilities|Casting|CastToBP_SaveGame _returnvalue))
  (bind _output_get (Variables|Default|SetSaveGameRef _asbp_save_game))
  (return (Variables|/Game/EndlessRun/Blueprints/SaveGame/old/BP_SaveGame.BP_SaveGame_C|GetRankingData _output_get)))