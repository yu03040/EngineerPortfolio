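; AI enemy character that carries a socket-attached weapon, senses the player and fires a rifle at them.
; AI Perception passes target and line-of-sight updates to the controller's blackboard, with a timer for delayed target loss.
; While alive, attacks read DT_Weapon's Rifle row for effects and spawned ammunition, and apply damage through a debug-drawn line trace.
; A timeline interpolates walk speed toward requested values.
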(event OnTargetPerceptionUpdated(AIPerception)
  (params (Actor :type Actor%20Object%20Reference) (Stimulus :type AI%20Stimulus%20Structure))
  (bind _output_get (Variables|Default|SetReceivedActor Actor))
  (if (Math|Boolean|ANDBoolean (== _output_get (Variables|Default|GetPlayer)) (Utilities|Struct|BreakAIStimulus Stimulus) (Variables|Default|GetIsAlive))
    ;[0 0 0] 見つけたものをセット
    (Variables|Default|SetReceivedActor (Variables|Default|GetPlayer))
    ;[0 0 0] 時間をリセット
    (Utilities|Time|ClearandInvalidateTimerbyHandle (Variables|Default|GetTargetLostTime))
    ;[0 0 0] ブラックボードにアクターの情報をセット
    (Class|EnemyAIControllerInterface|UpdateTargetActorKey(Message) (Variables|Default|GetEnemyController) (Variables|Default|GetReceivedActor))
    ;[0 0 0] 視界に入ったフラグをセット
    (Class|EnemyAIControllerInterface|UpdateHasLineOfSightKey(Message) (Variables|Default|GetEnemyController) true)
    (elif (== (Variables|Default|GetPlayer) (Variables|Default|GetReceivedActor))
      (bind _returnvalue (Utilities|Time|SetTimerbyEvent (EventDispatchers|CreateEvent :!event Custom|LostTarget) 5.0))
      (Variables|Default|SetTargetLostTime _returnvalue)
      ;[0 0 0] 視界に入っていないフラグをセット
      (Class|EnemyAIControllerInterface|UpdateHasLineOfSightKey(Message) (Variables|Default|GetEnemyController) false))))

(event Custom|LostTarget
  ;[0 0 0] ブラックボードにアクターの情報をセット
  ;;[0 0 0] 見つけていないので Target Actorは NULL
  (Class|EnemyAIControllerInterface|UpdateTargetActorKey(Message) (Variables|Default|GetEnemyController)))

(event EventBeginPlay
  (Transformation|AttachComponentToComponent (Variables|Default|GetWeapon) (Variables|Character|GetMesh) "Weapon_hand_rソケット" "KeepRelative" "KeepRelative" "KeepRelative" true))

(event EventChangeRunningSpeed
  (params (Speed :type Float%20%28single-precision%29))
  (Timeline|UpdateTimeLine PlayFromStart
    (:Update
      (Variables|/Script/Engine.CharacterMovementComponent|SetMaxWalkSpeed (Variables|Character|GetCharacterMovement) (Math|Interpolation|FInterpTo (Variables|/Script/Engine.CharacterMovementComponent|GetMaxWalkSpeed (Variables|Character|GetCharacterMovement)) Speed (Utilities|Time|GetWorldDeltaSeconds) 5.0)))))

(event EventAttackCharacter
  ;[0 0 0] 生きているか
  (if (Variables|Default|GetIsAlive)
    ;[0 0 0] ライフルでの攻撃
    (bind _returnvalue (Utilities|GetDataTableRow "/Game/ArmedWeapon/DT_Weapon.DT_Weapon" "Rifle")
      (:then
        (Variables|Default|SetGunshot%20Sound (.GunshotSound (Utilities|Struct|BreakWeaponStructure _returnvalue)))
        (Variables|Default|SetMuzzle%20Fire (.MuzzleFire (Utilities|Struct|BreakWeaponStructure _returnvalue)))
        (Variables|Default|SetMuzzle%20Fire%20Soket%20Name (.MuzzleFireSoketName (Utilities|Struct|BreakWeaponStructure _returnvalue)))
        (Variables|Default|SetFiring%20Montage (.FiringMontage (Utilities|Struct|BreakWeaponStructure _returnvalue)))
        (Variables|Default|SetAmmunition%20Class (.AmmunitionClass (Utilities|Struct|BreakWeaponStructure _returnvalue)))
        (Variables|Default|SetAmmunition%20Socket%20Name (.AmmunitionSocketName (Utilities|Struct|BreakWeaponStructure _returnvalue)))
        (Utilities|FlowControl|Sequence
          (:then_0
            (Audio|PlaySound2D (Variables|Default|GetGunshot%20Sound) 1.0 1.0 0.0 0 0))
          (:then_1
            (Animation|PlayAnimMontage (Variables|Default|GetFiring%20Montage) 0.1 "None"))
          (:then_2
            (Effects|SpawnEmitterAttached (Variables|Default|GetMuzzle%20Fire) (Variables|Default|GetWeapon) (Variables|Default|GetMuzzle%20Fire%20Soket%20Name)))
          (:then_3
            (Game|SpawnActorfromClass (Variables|Default|GetAmmunition%20Class) (Transformation|GetSocketTransform (Variables|Default|GetWeapon) (Variables|Default|GetMuzzle%20Fire%20Soket%20Name) "RTS_World") "AlwaysSpawn" "SelectDefaultAtRuntime" 0 0)
            (bind _outhit (Collision|LineTraceByChannel (Transformation|GetSocketLocation (Variables|Default|GetWeapon) (Variables|Default|GetAmmunition%20Socket%20Name)) (+ (Transformation|GetSocketLocation (Variables|Default|GetWeapon) (Variables|Default|GetAmmunition%20Socket%20Name)) (* (Math|Vector|GetForwardVector (Transformation|GetSocketRotation (Variables|Default|GetWeapon) (Variables|Default|GetMuzzle%20Fire%20Soket%20Name))) 1e+04)) "TraceTypeQuery1" false 0 "ForDuration" true "(R=1.000000,G=0.000000,B=0.000000,A=0.000000)" "(R=0.000000,G=1.000000,B=0.000000,A=1.000000)" 0.1))
            (if (== (.HitActor (Collision|BreakHitResult _outhit)) (Variables|Default|GetPlayer))
              (Game|Damage|ApplyDamage (Variables|Default|GetPlayer) 1e+01 0 0))))))))

(fn ConstructionScript)