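; BP_PathB_AIEnemyTarget is a spawn point that endlessly generates BP_PathB_AIEnemy pawns at its own location and rotation.
; On BeginPlay it starts InfiniteEnemyAIGeneration, which loops on a random delay of a few seconds, spawning each enemy with the BT_PatrolAI behavior tree and incrementing EnemyCount.
; The EnemyCount limit is checked only before the loop starts, so spawning itself is uncapped.
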(event EventBeginPlay
  (if (<= (Variables|Default|GetEnemyCount) 10)
    (Utilities|InfiniteEnemyAIGeneration)))

(fn ConstructionScript)