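; BP_AIEnemyController is an enemy AI controller that starts the BT_PatrolAI behavior tree on BeginPlay.
; An unconnected shooting chain would line trace forward from a living BP_AIEnemy pawn, play fire sound and explosion effects, and damage the player on a hit.
; That chain never runs, and the Damaged event is empty, so the behavior tree launch is the only active logic.
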(event EventBeginPlay
  (AI|RunBehaviorTree "/Game/Enemy/BT_PatrolAI.BT_PatrolAI"))

(event EventDamaged)

(fn ConstructionScript)